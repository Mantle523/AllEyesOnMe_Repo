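; First-person player character with walking, sprinting, crouching, cover-triggered crouch and mantling, driven by an FPS_Redux child actor.
; BeginPlay overrides that actor's tuning variables.
; Tick feeds it input, facing, ground traces and curve-sampled crouch and sprint progress, then applies its speed, FOV, camera height and motion outputs.
; Forward traces detect scalable walls; mantling switches to Flying and turns forward input upward, while key presses detect gamepad or mouse-and-keyboard aiming.
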(event `self.ReceiveBeginPlay`
  ;[0.3 0.5 0.8] Set/Edit Variables
  ;;[0.3 0.55 0.9] Ground Motion Variable Overrides
  (bind _asfps_redux (cast `FPS_Redux` (`ChildActorComponent.ChildActor` (`self.FPS_Redux`))))
  (`FPS_Redux.OverrideGroundVariables` _asfps_redux 1200.0 0.4 0.6 0.2 0.04)
  ;;[0.3 0.55 0.9] Aerial Motion Variable Overrides
  (`FPS_Redux.OverrideAerialVariables` _asfps_redux 0.6 0.0 0.3)
  ;;[0.3 0.55 0.9] Cover Variable Overrides
  (`FPS_Redux.OverrideCoverVariables` _asfps_redux -40.0 0.6 0.7 0.3 0.6)
  ;;[0.3 0.55 0.9] Sprint Variable Overrides
  (`FPS_Redux.OverrideSprintVariables` _asfps_redux 1.35 0.6 0.9 0.95)
  ;;[0.3 0.55 0.9] Detection Variable Overrides
  (`FPS_Redux.OverrideDetectionVariables` _asfps_redux 0.6)
  ;;[0.3 0.55 0.9] Aim Variable Overrides
  (`FPS_Redux.OverrideAimVariables` _asfps_redux 0.8)
  ;[0.6 0.3 0.6] Get Player Head Position
  (`FPS_Redux.CrouchOriginPosition` _asfps_redux (`.Z` (`KismetMathLibrary.BreakVector3f` (`SceneComponent.RelativeLocation` (`self.Camera_Container`)))))
  ;[0.6 0.3 0.6] Get original FOV
  (`FPS_Redux.FovOriginAngle` _asfps_redux (`CameraComponent.FieldOfView` (`self.Camera`)))
  ;[0.6 0.3 0.6] Ensures correct player height
  (`FPS_Redux.CrouchInput` _asfps_redux)
  (`FPS_Redux.CrouchInput` _asfps_redux))

(event `self.ReceiveTick`
  (params (DeltaSeconds :type "Float (single-precision)"))
  (bind _returnvalue (`GameplayStatics.GetPlayerController` 0))
  (bind _returnvalue_2 (`self.K2_GetActorRotation`))
  (bind _returnvalue_3 (`self.GetInputAxisValue`))
  (bind _returnvalue_4 (`self.GetInputAxisValue`))
  (bind _camera (`self.Camera`))
  (bind _camera_2 (`self.Camera`))
  (bind _capsulecomponent (`self.CapsuleComponent`))
  (bind _camera_3 (`self.Camera`))
  (bind _returnvalue_5 (`SceneComponent.GetRightVector` _camera))
  (bind _returnvalue_6 (`KismetMathLibrary.GetForwardVector` _returnvalue_2))
  (bind _returnvalue_7 (`KismetMathLibrary.GetUpVector` _returnvalue_2))
  (bind _returnvalue_8 (`SceneComponent.K2_GetComponentLocation` _capsulecomponent))
  (bind _returnvalue_9 (`SceneComponent.K2_GetComponentRotation` _capsulecomponent))
  (bind _returnvalue_10 (`KismetMathLibrary.MakeVector2D` (`self.GetInputAxisValue`) (`self.GetInputAxisValue`)))
  (bind _returnvalue_11 (* (`self.GetInputAxisValue`) -2.5))
  (bind _returnvalue_12 (* (`self.GetInputAxisValue`) -2.5))
  (bind _returnvalue_13 (`KismetMathLibrary.MakeRotator` 0.0 0.0 (.yaw (`self.K2_GetActorRotation`))))
  (bind _returnvalue_14 (`KismetMathLibrary.GetForwardVector` (`SceneComponent.K2_GetComponentRotation` _capsulecomponent)))
  (bind _returnvalue_15 (+ _returnvalue_8 (0.0 0.0 -20.0)))
  (bind _returnvalue_16 (+ _returnvalue_8 (0.0 0.0 -20.0)))
  (bind _returnvalue_17 (+ _returnvalue_8 (0.0 0.0 -100.0)))
  (bind _returnvalue_18 (* (`KismetMathLibrary.GetForwardVector` _returnvalue_9) 70.0))
  ;[0.6 0.3 0.6] Record deltaTime and Character Facing
  (bind _asfps_redux (cast `FPS_Redux` (`ChildActorComponent.ChildActor` (`self.FPS_Redux`))))
  (`FPS_Redux.TimeDifference` _asfps_redux DeltaSeconds)
  (bind _output_get (set `self.As FPS Redux` _asfps_redux))
  ;[0.4219 0.8438 0.4219] Is player currently mantling?
  (if (`FPS_Redux.IsMantling` _output_get)
    (`KismetSystemLibrary.PrintText` "Manling")
    (if (`|EnumInequality` (`CharacterMovementComponent.MovementMode` (`self.CharacterMovement`)) (`self.MovementMode`))
      (`CharacterMovementComponent.SetMovementMode` (`self.CharacterMovement`) "MOVE_Flying" 0))
    ;[0.4219 0.8438 0.4219] Behaviour While Mantling
    ;;[0.1328 0.2656 0.1328] Is the Player Facing Wall?
    (bind (_outhit _returnvalue_19) (`KismetSystemLibrary.LineTraceSingle` :`Start` _returnvalue_16 :`End` (+ _returnvalue_16 _returnvalue_18) :`TraceChannel` "TraceTypeQuery4" :`DrawDebugType` "ForDuration"))
    (if _returnvalue_19
      ;[0.7 0.7 3.674] Result
      ;;[0.4 0.4 0.7] Player Mantling
      (set `self.Mantling` true :!label _label)
      (else
        ;;[0.1328 0.2656 0.1328] Is the Wall Just Beneath Them?
        (bind (_outhit_2 _returnvalue_20) (`KismetSystemLibrary.LineTraceSingle` :`Start` _returnvalue_17 :`End` (+ _returnvalue_18 _returnvalue_17) :`TraceChannel` "TraceTypeQuery1" :`DrawDebugType` "ForDuration"))
        (if _returnvalue_20
          (goto _label)
          (else
            (`CharacterMovementComponent.SetMovementMode` (`self.CharacterMovement`) "MOVE_Walking" 0)
            (`KismetSystemLibrary.PrintString` "Mantle Ends")
            ;;[0.4 0.4 0.7] Player Not Mantling
            (`FPS_Redux.DisableMantle` _output_get)
            (set `self.Mantling` false :!label _label_2)))))
    (else
      ;[0.3 0.6 0.3] Raycast for Ground Detection
      (bind (_outhit_3 _returnvalue_21) (`KismetSystemLibrary.LineTraceSingle` _returnvalue_8 (+ _returnvalue_8 (* (`KismetMathLibrary.GetUpVector` _returnvalue_9) -95.0)) "TraceTypeQuery3"))
      (if (not _returnvalue_21)
        (`KismetSystemLibrary.PrintText` "Player Airborne"))
      (`FPS_Redux.GroundDetection` _output_get _returnvalue_21)
      ;[0.4219 0.8438 0.4219] Mantle Check Behaviour on Ground
      ;;[0.1328 0.2656 0.1328] Raycast forward from player's waist for "Scalable" objects
      (bind (_outhit_4 _returnvalue_22) (`KismetSystemLibrary.LineTraceSingle` _returnvalue_15 (+ _returnvalue_15 (* _returnvalue_14 70.0)) "TraceTypeQuery4"))
      ;;[0.1328 0.2656 0.1328] Did it hit something + is the player travelling towards it?
      (if _returnvalue_22
        (bind (_x _y) (`KismetMathLibrary.BreakVector3f` (`FPS_Redux.lastDirection` _output_get)))
        (if (>= (`FPS_Redux.returnTolerance` _output_get) (`KismetMathLibrary.DegAcos` (`KismetMathLibrary.Dot_VectorVector` (`KismetMathLibrary.Normal` (`KismetMathLibrary.MakeVector` _x _y)) (`KismetMathLibrary.GetForwardVector` _returnvalue_9))))
          (`FPS_Redux.OnTickMantle` _output_get _returnvalue_14)
          (goto _label_2)
          (else
            _)))
      (`FPS_Redux.ResetMantle` _output_get)
      (goto _label_2)))
  ;[0.4219 0.8438 0.4219] Check whether player is moving between crouch states, and in what direction
  (if (`FPS_Redux.IsCrouching` _output_get)
    (if (`FPS_Redux.CrouchType` _output_get)
      (`FPS_Redux.CrouchDisplacement` _output_get (`CurveFloat.GetFloatValue` (`self.Crouch Curve`) (`KismetMathLibrary.FClamp` (`FPS_Redux.CrouchProgress` _output_get))))
      (else
        (`FPS_Redux.CrouchDisplacement` _output_get (`CurveFloat.GetFloatValue` (`self.Uncrouch Curve`) (`KismetMathLibrary.FClamp` (`FPS_Redux.UncrouchProgress` _output_get)))))))
  ;[0.4219 0.8438 0.4219] Check whether the player is moving between sprint states, and in what direction
  (if (`FPS_Redux.IsSprinting` _output_get)
    (if (`FPS_Redux.IsAccelerating` _output_get)
      (`FPS_Redux.SprintDisplacement` _output_get (`CurveFloat.GetFloatValue` (`self.AccSprint Curve`) (`KismetMathLibrary.FClamp` (`FPS_Redux.AccelerateSprintProgress` _output_get))))
      (else
        (`FPS_Redux.SprintDisplacement` _output_get (`CurveFloat.GetFloatValue` (`self.DecSprint Curve`) (`KismetMathLibrary.FClamp` (`FPS_Redux.DecelerateSprintProgress` _output_get)))))))
  ;[0.7 0.7 3.674] Player is using a controller?
  (if (`FPS_Redux.InputTypeController` _output_get)
    ;[0.7 0.7 3.674] Write inputs to script
    ;;[0.4 0.4 0.7] Gamepad Inputs
    (`FPS_Redux.ControlInputs` _output_get _returnvalue_10 (`KismetMathLibrary.MakeVector2D` _returnvalue_4 _returnvalue_11))
    (bind _returnvalue_23 (`FPS_Redux.ReturnXMultiplier` _output_get))
    ;[0.3 0.6 0.3] Per-Frame Aiming
    ;;[0.1328 0.2656 0.1328] Rotate Player Character Horizontally by Sensitivity
    (`self.AddControllerYawInput` (* _returnvalue_4 _returnvalue_23))
    (`Controller.SetControlRotation` _returnvalue _returnvalue_13)
    (bind _returnvalue_24 (`FPS_Redux.ReturnYMultiplier` _output_get))
    ;;[0.1328 0.2656 0.1328] Rotate Camera Vertically by Sensitivity
    (`SceneComponent.K2_AddLocalRotation` _camera_2 (`KismetMathLibrary.MakeRotator` 0.0 (* _returnvalue_11 _returnvalue_24)) false false)
    (else
      ;;[0.4 0.4 0.7] K&M Inputs
      (`FPS_Redux.ControlInputs` _output_get _returnvalue_10 (`KismetMathLibrary.MakeVector2D` _returnvalue_3 _returnvalue_12))
      (`self.AddControllerYawInput` (* _returnvalue_23 _returnvalue_3))
      (`Controller.SetControlRotation` _returnvalue _returnvalue_13)
      (`SceneComponent.K2_AddLocalRotation` _camera_2 (`KismetMathLibrary.MakeRotator` 0.0 (* _returnvalue_24 _returnvalue_12)) false false)))
  (`SceneComponent.K2_SetRelativeRotation` _camera_2 (`KismetMathLibrary.MakeRotator` 0.0 (`KismetMathLibrary.ClampAngle` (.pitch (`SceneComponent.K2_GetComponentRotation` _camera_2)) -80.0 80.0)) false false)
  ;[0.6 0.3 0.6] Get Facing After Camera Manipulation
  (bind _asfps_redux_2 (cast `FPS_Redux` (`ChildActorComponent.ChildActor` (`self.FPS_Redux`))))
  (`FPS_Redux.PerspectiveInput` _asfps_redux_2 (`SceneComponent.GetForwardVector` _camera_3) (`SceneComponent.GetRightVector` _camera_3))
  ;[0.3 0.6 0.3] Calculate Player's New Position (& FOV/Head Position
  (set `CharacterMovementComponent.MaxWalkSpeed` (`FPS_Redux.ReturnTopSpeed` _asfps_redux_2) (`self.CharacterMovement`))
  (`FPS_Redux.OnTickMotion` _asfps_redux_2)
  (`CameraComponent.SetFieldOfView` _camera (`FPS_Redux.FovOutput` _asfps_redux_2))
  (bind (_x_2 _y_2) (`KismetMathLibrary.BreakVector2D` (`FPS_Redux.MotionOutput` _asfps_redux_2)))
  (`self.AddMovementInput` _returnvalue_5 _x_2)
  (if (`self.Mantling`)
    (`self.AddMovementInput` _returnvalue_7 _y_2)
    (set `self.Y Axis Movement` (* _y_2 _returnvalue_7))
    (else
      (`self.AddMovementInput` _returnvalue_6 _y_2)
      (set `self.Y Axis Movement` (* _returnvalue_6 _y_2))
      (if (`FPS_Redux.AirborneState` _asfps_redux_2)
        (`self.AddMovementInput` _returnvalue_7 -9.81))))
  (`SceneComponent.K2_SetRelativeLocation` (`self.Camera_Container`) (`KismetMathLibrary.MakeVector` 0.0 0.0 (`FPS_Redux.CrouchOutput` _asfps_redux_2)) false true)
  (`FPS_Redux.RecordDirection` _asfps_redux_2 (+ (* _x_2 _returnvalue_5) (`self.Y Axis Movement`))))

(event `Key|AnyKey`
  (params (Key :type "Key Structure"))
  (bind _returnvalue (`KismetInputLibrary.Key_IsGamepadKey` Key))
  (bind _childactor (`ChildActorComponent.ChildActor` (`self.FPS_Redux`)))
  ;[0.2 0.6 0.6] Controller or Keyboard?
  (:`Pressed`
    (bind _asfps_redux (cast `FPS_Redux` _childactor))
    (if (!= (`FPS_Redux.InputTypeController` _asfps_redux) _returnvalue)
      (`FPS_Redux.InputType` _asfps_redux _returnvalue)
      (bind _asfps_redux_2 (cast `FPS_Redux` _childactor))
      (if (`FPS_Redux.InputTypeController` _asfps_redux_2)
        (`KismetSystemLibrary.PrintText` "Player using gamepad")
        (else
          (`KismetSystemLibrary.PrintText` "Player using M&K"))))))

(event `InputAction|Crouch`
  (params (Key :type "Key Structure"))
  ;[0.2 0.6 0.6] Toggling Crouch State
  (:`Pressed`
    (bind _asfps_redux (cast `FPS_Redux` (`ChildActorComponent.ChildActor` (`self.FPS_Redux`))))
    (`FPS_Redux.CrouchInput` _asfps_redux)
    (`KismetSystemLibrary.PrintString` (`FPS_Redux.CurrentCrouchState` _asfps_redux))))

(event `self.Cover Detection.OnComponentBeginOverlap`
  (params (OverlappedComponent :type "PrimitiveComponent Object Reference") (OtherActor :type "Actor Object Reference") (OtherComp :type "PrimitiveComponent Object Reference") (OtherBodyIndex :type Integer) (bFromSweep :type Boolean) (SweepResult :type "HitResult Structure (by ref)"))
  ;[0.2 0.6 0.6] Nearing cover
  (if (`ActorComponent.ComponentHasTag` OtherComp "Cover")
    (bind _asfps_redux (cast `FPS_Redux` (`ChildActorComponent.ChildActor` (`self.FPS_Redux`))))
    (`FPS_Redux.CrouchAdd` _asfps_redux)
    (`KismetSystemLibrary.PrintString` (`FPS_Redux.CurrentForcedCover` _asfps_redux))))

(event `self.Cover Detection.OnComponentEndOverlap`
  (params (OverlappedComponent :type "PrimitiveComponent Object Reference") (OtherActor :type "Actor Object Reference") (OtherComp :type "PrimitiveComponent Object Reference") (OtherBodyIndex :type Integer))
  ;[0.2 0.6 0.6] Drawing Away From Cover
  (if (`ActorComponent.ComponentHasTag` OtherComp "Cover")
    (bind _asfps_redux (cast `FPS_Redux` (`ChildActorComponent.ChildActor` (`self.FPS_Redux`))))
    (`FPS_Redux.CrouchSubtract` _asfps_redux)
    (`KismetSystemLibrary.PrintString` (`FPS_Redux.CurrentForcedCoverExit` _asfps_redux))))

(event `InputAction|Sprint`
  (params (Key :type "Key Structure"))
  (bind _childactor (`ChildActorComponent.ChildActor` (`self.FPS_Redux`)))
  ;[0.2 0.6 0.6] Sprinting
  (:`Pressed`
    (bind _asfps_redux (cast `FPS_Redux` _childactor))
    (`FPS_Redux.SprintActivation` _asfps_redux)
    (`KismetSystemLibrary.PrintText` "Beginning Sprint")
    (if (`FPS_Redux.IsAccelerating` _asfps_redux)
      (`KismetSystemLibrary.PrintText` "Set to accelerate")
      (else
        (`KismetSystemLibrary.PrintText` "Error in setting sprint state"))))
  (:`Released`
    (bind _asfps_redux_2 (cast `FPS_Redux` _childactor))
    (`FPS_Redux.SprintDectivation` _asfps_redux_2)
    (`KismetSystemLibrary.PrintText` "Ending Sprint")))

(fn `UserConstructionScript`
  (set `self.MovementMode` "MOVE_Flying"))